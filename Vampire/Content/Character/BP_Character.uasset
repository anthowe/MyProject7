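; BP_Character is a character Blueprint with Health, Stamina and Coins stats and a jump input.
; Pressing N lowers Health and raises Stamina and Coins, while the Jump action calls the built-in Jump.
; An unconnected sprint fragment, which never runs, would set IsSprinting on the ABP_Character anim instance and switch max walk speed between RunSpeed and WalkSpeed.
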(event EventBeginPlay)

(event Collision|EventActorBeginOverlap
  (params (OtherActor :type Actor%20Object%20Reference)))

(event EventTick
  (params (DeltaSeconds :type Float%20%28single-precision%29)))

(event Input|ActionEvents|InputActionSprint
  (params (Key :type Key%20Structure)))

(event Input|ActionEvents|InputActionJump
  (params (Key :type Key%20Structure))
  (:Pressed
    (Character|Jump)))

(event Input|KeyboardEvents|N
  (params (Key :type Key%20Structure))
  (:Pressed
    (Variables|Default|SetHealth (- (Variables|Default|GetHealth) 1e+01))
    (Variables|Default|SetStamina (+ (Variables|Default|GetStamina) 1e+01))
    (Variables|Default|SetCoins (+ (Variables|Default|GetCoins) 1))))

(fn ConstructionScript)